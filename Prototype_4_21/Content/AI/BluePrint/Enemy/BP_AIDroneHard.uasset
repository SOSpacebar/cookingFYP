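; BP_AIDroneHard is an enemy AI drone, apparently the hard variant, whose graph handles damage from projectiles.
; A hit by a FirstPersonProjectile destroys the bullet and applies a fixed amount of damage through TakeDamage.
; An overlap with a RocketProjectile applies that rocket's AoeDamagePoints, but only if its AOEDamage component overlaps the drone.
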(event `self.ReceiveHit`
  (params (MyComp :type "PrimitiveComponent Object Reference") (Other :type "Actor Object Reference") (OtherComp :type "PrimitiveComponent Object Reference") (bSelfMoved :type Boolean) (HitLocation :type "Vector Structure") (HitNormal :type "Vector Structure") (NormalImpulse :type "Vector Structure") (Hit :type "HitResult Structure (by ref)"))
  ;[1 1 1] Damage check on Enemy
  ;;[1 1 1] Check which projectile hit
  (bind _asfirst_person_projectile (cast `/Game/Interactables/FirstPersonProjectile` Other))
  (`self.K2_DestroyActor` _asfirst_person_projectile) ; Destroy the Bullet
  (`I_Damageable.TakeDamage` 10.0))

(event `self.ReceiveActorBeginOverlap`
  (params (OtherActor :type "Actor Object Reference"))
  ;[1 1 1] Damage check on Enemy
  ;;[1 1 1] Check which projectile hit
  (bind _asrocket_projectile (cast `/Game/Interactables/RocketProjectile` OtherActor))
  (if (`PrimitiveComponent.IsOverlappingActor` (`/Game/Interactables/RocketProjectile.AOEDamage` _asrocket_projectile) self)
    (`I_Damageable.TakeDamage` (`/Game/Interactables/RocketProjectile.AoeDamagePoints` _asrocket_projectile))))

(fn `UserConstructionScript`)