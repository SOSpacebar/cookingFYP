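; Spaceship emergency box with a hinged lid and two battery slots that restore the ship's lights.
; M releases the lid to physics; Tick snaps it back onto the box once constraint twist exceeds the limit.
; RepairBatteryEvent kills the lights and enables collision on the broken batteries.
; Slot overlaps attach unbroken batteries and destroy that collider, using the other's validity to choose half or full light.
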(event `self.ReceiveBeginPlay`
  (`self.SetActorEnableCollision` (`ChildActorComponent.ChildActor` (`self.BrokenBatteryLeft`)) false)
  (`self.SetActorEnableCollision` (`ChildActorComponent.ChildActor` (`self.BrokenBatteryRight`)) false))

(event `self.ReceiveTick`
  (params (DeltaSeconds :type "Float (single-precision)"))
  (if (`self.IsReleased`)
    (`self.SecureLockWhenOverLimit` 90.0)))

(event `Key|M`
  (params (Key :type "Key Structure"))
  (:`Pressed`
    (`self.ReleaseLock`)))

(event `self.BatteryColliderLeft.OnComponentBeginOverlap`
  (params (OverlappedComponent :type "PrimitiveComponent Object Reference") (OtherActor :type "Actor Object Reference") (OtherComp :type "PrimitiveComponent Object Reference") (OtherBodyIndex :type Integer) (bFromSweep :type Boolean) (SweepResult :type "HitResult Structure (by ref)"))
  (`self.SnapToLocation` (`self.BatteryColliderLeft`) OtherComp))

(event `self.BatteryColliderRight.OnComponentBeginOverlap`
  (params (OverlappedComponent :type "PrimitiveComponent Object Reference") (OtherActor :type "Actor Object Reference") (OtherComp :type "PrimitiveComponent Object Reference") (OtherBodyIndex :type Integer) (bFromSweep :type Boolean) (SweepResult :type "HitResult Structure (by ref)"))
  (`self.SnapToLocation` (`self.BatteryColliderRight`) OtherComp))

(fn `ReleaseLock`
  (`PrimitiveComponent.SetSimulatePhysics` (`self.EmergencyBoxLid`) true)
  (set `self.IsReleased` true))

(fn `RepairBatteryEvent`
  (`self.SetActorEnableCollision` (`ChildActorComponent.ChildActor` (`self.BrokenBatteryLeft`)) true)
  (`self.SetActorEnableCollision` (`ChildActorComponent.ChildActor` (`self.BrokenBatteryRight`)) true)
  (`/Game/BoonPingTest/Blueprints/Spaceship.AdjustLights` (`self.TheSpaceship`) 0.0))

(fn `SecureLockWhenOverLimit`
  (params (Limit :type "Float (double-precision)"))
  (bind _emergencyboxlid (`self.EmergencyBoxLid`))
  (if (> (`PhysicsConstraintComponent.GetCurrentTwist` (`self.PhysicsConstraint`)) Limit)
    (`PrimitiveComponent.SetSimulatePhysics` _emergencyboxlid false)
    (`SceneComponent.K2_AttachToComponent` _emergencyboxlid (`self.EmergencyBox`) "None" "SnapToTarget" "SnapToTarget" "SnapToTarget" false)
    (set `self.IsReleased` false)))

(fn `SnapToLocation`
  (params (TheBoxCollision :type "BoxComponent Object Reference") (TheComponent :type "PrimitiveComponent Object Reference (by ref)"))
  (bind _thespaceship (`self.TheSpaceship`))
  (bind _thespaceship_2 (`self.TheSpaceship`))
  (bind _asemergency_battery (cast `/Game/BoonPingTest/Blueprints/EmergencyBattery` (`ActorComponent.GetOwner` TheComponent)))
  (if (not (`/Game/BoonPingTest/Blueprints/EmergencyBattery.IsBroken` _asemergency_battery))
    ;[1 1 1] Left Collider
    (if (== TheBoxCollision (`self.BatteryColliderLeft`))
      (`PrimitiveComponent.SetSimulatePhysics` TheComponent false)
      (`PrimitiveComponent.SetCollisionEnabled` TheComponent "NoCollision")
      (`self.K2_AttachToComponent` (`ActorComponent.GetOwner` TheComponent) (`self.BatteryLocationLeft`) "None" "SnapToTarget" "SnapToTarget" "KeepRelative" true)
      (`ActorComponent.K2_DestroyComponent` (`self.BatteryColliderLeft`))
      (if (`KismetSystemLibrary.IsValid` (`self.BatteryColliderRight`))
        (`/Game/BoonPingTest/Blueprints/Spaceship.AdjustLights` _thespaceship_2 0.5)
        (else
          (`ActorComponent.Deactivate` (`self.TheEmitter`))
          (`/Game/BoonPingTest/Blueprints/Spaceship.AdjustLights` _thespaceship_2 1.0)))
      (else
        ;[1 1 1] Right Collider
        (if (== TheBoxCollision (`self.BatteryColliderRight`))
          (`PrimitiveComponent.SetSimulatePhysics` TheComponent false)
          (`PrimitiveComponent.SetCollisionEnabled` TheComponent "NoCollision")
          (`self.K2_AttachToComponent` (`ActorComponent.GetOwner` TheComponent) (`self.BatteryLocationRight`) "None" "SnapToTarget" "SnapToTarget" "KeepRelative" true)
          (`ActorComponent.K2_DestroyComponent` (`self.BatteryColliderRight`))
          (if (`KismetSystemLibrary.IsValid` (`self.BatteryColliderLeft`))
            (`/Game/BoonPingTest/Blueprints/Spaceship.AdjustLights` _thespaceship 0.5)
            (else
              (`ActorComponent.Deactivate` (`self.TheEmitter`))
              (`/Game/BoonPingTest/Blueprints/Spaceship.AdjustLights` _thespaceship 1.0))))))))

(fn `UserConstructionScript`)