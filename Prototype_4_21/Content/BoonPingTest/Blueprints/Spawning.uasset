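; Spawning actor Blueprint that animates a material fade on a mesh and destroys itself when the timeline finishes.
; SetSpawnMaterial creates and stores a dynamic material instance from the first material of a supplied mesh.
; TriggerSpawn or the X key flips between playing the timeline forward and in reverse, with updates lerping the material's "fadeout" scalar from one toward zero as the track rises.
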(event `self.ReceiveBeginPlay`)

(event `TriggerSpawn`
  (`/Engine/EditorBlueprintResources/StandardMacros.FlipFlop` :!label _label
    (:`A`
      (bind (_direction _newtrack_0) (`Timeline|Timeline_0` :!via `PlayFromStart` :!label _label_2)
        (:`Update`
          (`MaterialInstanceDynamic.SetScalarParameterValue` (`self.DynamicMaterial`) "fadeout" (`KismetMathLibrary.Lerp` 1.0 0.0 _newtrack_0)))
        (:`Finished`
          (`self.K2_DestroyActor`))))
    (:`B`
      (goto _label_2 :!via `ReverseFromEnd`))))

(event `Key|X`
  (params (Key :type "Key Structure"))
  (:`Pressed`
    (goto _label)))

(fn `SetSpawnMaterial`
  (params (TheMesh :type "PrimitiveComponent Object Reference (by ref)"))
  (bind _returnvalue (`PrimitiveComponent.CreateDynamicMaterialInstance` TheMesh 0 (`PrimitiveComponent.GetMaterial` TheMesh 0) "None"))
  (set `self.DynamicMaterial` _returnvalue))

(fn `UserConstructionScript`)