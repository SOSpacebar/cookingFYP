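; Pistol2 is a hitscan pistol with haptic feedback that damages AI drones.
; On BeginPlay it sets its spawn material and initializes.
; Fire runs an ammo check, then plays a left-hand haptic effect, updates the gun state and line-traces forward from the muzzle for one object type, with debug drawing on.
; A hit BP_AIDrone receives fixed damage through its TakeDamage call.
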(event `self.ReceiveBeginPlay`
  (`self.SetSpawnMaterial`)
  (`self.Init`))

(event `self.Fire`
  (bind _muzzle (`self.Muzzle`))
  (bind _returnvalue (`SceneComponent.K2_GetComponentLocation` _muzzle))
  (bind _hasammo (`self.AmmoCheckAndAppend`))
  (if _hasammo
    (`PlayerController.PlayHapticEffect` (`GameplayStatics.GetPlayerController` 0) "/Game/BoonPingTest/NewHapticFeedbackEffect_Curve.NewHapticFeedbackEffect_Curve" "Left" 1.0 false)
    (set `self.GunState` "NewEnumerator1")
    (bind _outhit (`KismetSystemLibrary.LineTraceSingleForObjects` :`Start` _returnvalue :`End` (+ (* (`SceneComponent.GetForwardVector` _muzzle) 1000) _returnvalue) :`ObjectTypes` (`|MakeArray` "ObjectTypeQuery9" :!type "EObjectTypeQuery Enum") :`DrawDebugType` "ForDuration" :`DrawTime` 2.0))
    (bind _asbp_aidrone (cast `/Game/AI/BluePrint/BP_AIDrone` (`.HitActor` (`GameplayStatics.BreakHitResult` _outhit))))
    (`I_Damageable.TakeDamage` _asbp_aidrone 50.0)))

(fn `UserConstructionScript`)