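; VR rocket launcher weapon that locks onto AI drones while the trigger is held and fires a rocket on release.
; While held, Tick line-traces from the laser sight and highlights the live drone it hits with custom depth.
; Once TriggerHeld clears, it checks ammo, plays haptics on the holding hand, spawns a rocket at the muzzle and passes any valid target with health for homing.
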(event `self.ReceiveBeginPlay`
  (`self.SetSpawnMaterial`))

(event `self.Fire`
  (params (HandDirection :type Boolean))
  ;[1 1 1] Rocket Functions
  (set `self.TriggerHeld` true))

(event `self.ReceiveTick`
  (params (DeltaSeconds :type "Float (single-precision)"))
  (bind _returnvalue (`GameplayStatics.GetPlayerController` 0))
  (bind _lasersight (`self.LaserSight`))
  (bind _homingtarget_2 (`self.HomingTarget_2`))
  (bind _homingtarget_2_2 (`self.HomingTarget_2`))
  (bind _muzzle (`self.Muzzle`))
  (bind _returnvalue_2 (`SceneComponent.K2_GetComponentLocation` _lasersight))
  (bind _mesh (`Character.Mesh` _homingtarget_2))
  ;[1 1 1] Rocket Functions
  (if (`self.TriggerHeld`)
    ;;[1 1 1] Targeting Laser
    (set `self.TriggerForFire` true)
    (bind (_outhit _returnvalue_3) (`KismetSystemLibrary.LineTraceSingleForObjects` :`Start` _returnvalue_2 :`End` (+ _returnvalue_2 (* (`SceneComponent.GetForwardVector` _lasersight) 5000.0)) :`ObjectTypes` (`self.ObjectsTarget`) :`DrawDebugType` "ForOneFrame"))
    (if _returnvalue_3
      (bind _asaidrone (cast `AIDrone` (`.HitActor` (`GameplayStatics.BreakHitResult` _outhit))))
      (if (not (`AIDrone.isDead` _asaidrone))
        (`/Engine/EditorBlueprintResources/StandardMacros.IsValid` _homingtarget_2
          (:`Is Valid`
            (`PrimitiveComponent.SetRenderCustomDepth` _mesh false))
          (:`Is Not Valid`
            _))
        (bind _output_get (set `self.HomingTarget_2` _asaidrone))
        (if (not (`AIDrone.isDead` _asaidrone))
          (bind _mesh_2 (`Character.Mesh` _output_get))
          (`PrimitiveComponent.SetRenderCustomDepth` _mesh_2 true)
          (`KismetSystemLibrary.Delay` 2.0)
          (`PrimitiveComponent.SetRenderCustomDepth` _mesh_2 false)))
      (else
        (`/Engine/EditorBlueprintResources/StandardMacros.IsValid` _homingtarget_2
          (:`Is Valid`
            (`PrimitiveComponent.SetRenderCustomDepth` _mesh false)))))
    (elif (`self.TriggerForFire`)
      ;;[1 1 1] Fire Rocket
      (bind _hasammo (`self.AmmoCheckAndAppend`))
      (if _hasammo
        (if (`self.This Hand Direction`)
          (`PlayerController.PlayHapticEffect` _returnvalue "/Game/Weapons/NewHapticFeedbackEffect_Curve.NewHapticFeedbackEffect_Curve" "Left" 1.0 false)
          (else
            (`PlayerController.PlayHapticEffect` _returnvalue "/Game/Weapons/NewHapticFeedbackEffect_Curve.NewHapticFeedbackEffect_Curve" "Right" 1.0 false)))
        (bind _returnvalue_4 (`|SpawnActorFromClass` "/Game/Weapons/Blueprints/RocketProjectile.RocketProjectile_C" (`KismetMathLibrary.MakeTransform` (`SceneComponent.K2_GetComponentLocation` _muzzle) (`SceneComponent.K2_GetComponentRotation` _muzzle)) "Undefined" "OverrideRootScale" null null))
        (`GameplayStatics.PlaySoundAtLocation` "/Game/Audio/Gun/Rocket_Cue.Rocket_Cue" (`self.K2_GetActorLocation`) (struct) 1.0 1.0 0.0 null null null) ; Play firing sound
        (set `self.TriggerForFire` false)
        (`/Engine/EditorBlueprintResources/StandardMacros.IsValid` _homingtarget_2_2
          (:`Is Valid`
            (if (not (== (`AIDrone.health` _homingtarget_2_2) 0.0))
              (`/Game/Weapons/Blueprints/RocketProjectile.HomingRocket` _returnvalue_4 (`self.ActorHomingTarget`) (`self.HomingTarget`) null _homingtarget_2_2))))))))

(fn `UserConstructionScript`)