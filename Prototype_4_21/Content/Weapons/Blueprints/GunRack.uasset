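; Gun rack actor that displays a pistol, SMG, rocket launcher and shield, and replenishes them via RespawnGun.
; RespawnGun detaches the passed item, spawns a new actor of the same class and calls its Spawn.
; Class checks and a Shield cast fallback attach the replacement to its matching holder with a hand-tuned offset.
; Tick rotates the four circle components by a fixed step per frame, without delta-time scaling.
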(event `self.ReceiveTick`
  (params (DeltaSeconds :type "Float (single-precision)"))
  (`SceneComponent.K2_AddLocalRotation` (`self.PistolCircle`) (struct :`Pitch` 1.0) false false)
  (`SceneComponent.K2_AddLocalRotation` (`self.SmgCircle`) (struct :`Pitch` 1.0) false false)
  (`SceneComponent.K2_AddLocalRotation` (`self.RocketLauncherCircle`) (struct :`Pitch` 1.0) false false)
  (`SceneComponent.K2_AddLocalRotation` (`self.ShieldCircle`) (struct :`Pitch` 1.0) false false))

(fn `RespawnGun`
  (params (TheGun :type "Actor Object Reference (by ref)"))
  (locals (NewLocalVar_0 :type "EAttachmentRule Enum" :default "KeepRelative"))
  (bind _returnvalue (`GameplayStatics.GetObjectClass` TheGun))
  (`SceneComponent.K2_DetachFromComponent` (`Actor.RootComponent` TheGun) "KeepRelative" "KeepRelative" "KeepWorld" true)
  (bind _returnvalue_2 (`|SpawnActorFromClass` _returnvalue (`KismetMathLibrary.MakeTransform` (0.0 0.0 0.0)) "Undefined" "OverrideRootScale" null null))
  (bind _asgun (cast `/Game/Weapons/Blueprints/Gun` _returnvalue_2)
    (:`then`
      (`/Game/SpaceShip/Blueprints/SpawningSkeletalMesh.Spawn` _asgun)
      (if (== _returnvalue "/Game/Weapons/Blueprints/Pistol2.Pistol2_C")
        (`self.K2_AttachToComponent` _returnvalue_2 (`self.PistolHolder`) "None" "KeepRelative" "KeepRelative" "KeepRelative" true)
        (`self.K2_SetActorRelativeLocation` _returnvalue_2 (0.0 0.0 -10.0) false false)
        (elif (== _returnvalue "/Game/Weapons/Blueprints/SMG2.SMG2_C")
          (`self.K2_AttachToComponent` _returnvalue_2 (`self.SmgHolder`) "None" "KeepRelative" "KeepRelative" "KeepRelative" true)
          (`self.K2_SetActorRelativeLocation` _returnvalue_2 (0.0 0.0 -10.0) false false)
          (elif (== _returnvalue "/Game/Weapons/Blueprints/RocketLauncher_2.RocketLauncher_2_C")
            (`self.K2_AttachToComponent` _returnvalue_2 (`self.RocketLauncherHolder`) "None" "KeepRelative" "KeepRelative" "KeepRelative" true)
            (`self.K2_SetActorRelativeTransform` _returnvalue_2 (`KismetMathLibrary.MakeTransform` (10.5 -5.5 0.0) (struct :`Pitch` 90.0)) false false)))))
    (:`CastFailed`
      (bind _asshield (cast `/Game/Weapons/Blueprints/Shield` _returnvalue_2))
      (`/Game/SpaceShip/Blueprints/SpawningStaticMesh.Spawn` _asshield)
      (`self.K2_AttachToComponent` _returnvalue_2 (`self.ShieldHolder`) "None" "KeepRelative" "KeepRelative" "KeepRelative" true)
      (`self.K2_SetActorRelativeTransform` _returnvalue_2 (`KismetMathLibrary.MakeTransform` (0.0 -5.6 -1.0) (struct :`Yaw` 90.0)) false false))))

(fn `UserConstructionScript`)