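; Submachine gun weapon Blueprint that fires automatically while the trigger is held.
; An IsTriggerPressed event opens a gate that spawns a FirstPersonProjectile at MuzzleLocation with a firing sound, then re-enters itself through a RateOfFire retriggerable delay.
; Pressing sets GunFiring and hides the SubmachineGun component.
; Release clears the flag at once, then unhides the component and closes the gate after a short delay.
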(event `/Game/Weapons/Blueprints/GunInterface.IsTriggerPressed`
  (params (IsPressed :type Boolean))
  (bind _muzzlelocation (`self.MuzzleLocation`))
  (if IsPressed
    (set `self.GunFiring` true)
    (`SceneComponent.SetHiddenInGame` (`self.SubmachineGun`) true false)
    (`|ExecutionSequence`
      (:`then_0`
        (goto _label :!via `Open`))
      (:`then_1`
        (`/Engine/EditorBlueprintResources/StandardMacros.Gate` true :!label _label
          (:`Exit`
            (`|ExecutionSequence`
              (:`then_0`
                (`|SpawnActorFromClass` "/Game/Weapons/Blueprints/FirstPersonProjectile.FirstPersonProjectile_C" (`KismetMathLibrary.MakeTransform` (`SceneComponent.K2_GetComponentLocation` _muzzlelocation) (`SceneComponent.K2_GetComponentRotation` _muzzlelocation)) "Undefined" "OverrideRootScale" null null)
                (`GameplayStatics.PlaySoundAtLocation` "/Game/Audio/Gun/GunFire_Cue.GunFire_Cue" (`self.K2_GetActorLocation`) (struct) 1.0 1.0 0.0 null null null) ; Play firing sound
              )
              (:`then_1`
                (`KismetSystemLibrary.RetriggerableDelay` (`self.RateOfFire`))
                (goto _label)))))))
    (else
      (set `self.GunFiring` false)
      (`KismetSystemLibrary.Delay` 0.2)
      (`SceneComponent.SetHiddenInGame` (`self.SubmachineGun`) false false)
      (goto _label :!via `Close`))))

(fn `UserConstructionScript`)