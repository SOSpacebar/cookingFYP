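; Base gun Blueprint that tracks ammo and shows the remaining count on a text render component.
; Init writes the starting count, and AmmoCheckAndAppend spends one round, updates the text and returns true when GunState is in its first state and ammo remains.
; An empty gun turns the text red and returns false, as does any other state.
; Fire takes a hand direction but is empty here, and the event graph does nothing.
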(event `self.ReceiveBeginPlay`)

(fn `AmmoCheckAndAppend`
  (returns (HasAmmo :type Boolean))
  (bind _ammo (`self.Ammo`))
  (if (`|EnumEquality` (`self.GunState`) "NewEnumerator0")
    (if (!= _ammo 0)
      (bind _result (`/Engine/EditorBlueprintResources/StandardMacros.DecrementInt` _ammo)
        (:`  `
          (`TextRenderComponent.K2_SetText` (`self.TextRender`) (`KismetTextLibrary.Conv_IntToText` _result))
          (return true)))
      (else
        (`TextRenderComponent.SetTextRenderColor` (`self.TextRender`) (make `Color` 0 0 200 1)))))
  (return false))

(fn `Fire`
  (params (HandDirection :type Boolean)))

(fn `Init`
  (`TextRenderComponent.K2_SetText` (`self.TextRender`) (`KismetTextLibrary.Conv_IntToText` (`self.Ammo`))))

(fn `UserConstructionScript`)