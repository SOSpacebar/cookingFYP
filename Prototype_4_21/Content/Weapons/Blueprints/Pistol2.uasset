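; VR pistol weapon that fires a hitscan shot and damages AI drones.
; On begin play it sets its spawn material and runs its init.
; Fire passes an ammo check, then sets the gun state, pulses haptics in the firing hand and plays muzzle sound, flash and bullet effects.
; A line trace from the muzzle places impact sparks and applies fixed damage to any drone it hits.
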(event `self.ReceiveBeginPlay`
  (`self.SetSpawnMaterial`)
  (`self.Init`))

(event `self.ReceiveTick`
  (params (DeltaSeconds :type "Float (single-precision)")))

(event `self.Fire`
  (params (HandDirection :type Boolean))
  (bind _returnvalue (`GameplayStatics.GetPlayerController` 0))
  (bind _muzzle (`self.Muzzle`))
  (bind _muzzle_2 (`self.Muzzle`))
  (bind _returnvalue_2 (`SceneComponent.K2_GetComponentLocation` _muzzle_2))
  (bind _hasammo (`self.AmmoCheckAndAppend`))
  (if _hasammo
    (if HandDirection
      (`PlayerController.PlayHapticEffect` _returnvalue "/Game/Weapons/NewHapticFeedbackEffect_Curve.NewHapticFeedbackEffect_Curve" "Left" 1.0 false)
      (else
        (`PlayerController.PlayHapticEffect` _returnvalue "/Game/Weapons/NewHapticFeedbackEffect_Curve.NewHapticFeedbackEffect_Curve" "Right" 1.0 false)))
    (set `self.GunState` "NewEnumerator1")
    (`GameplayStatics.PlaySoundAtLocation` "/Game/Audio/Gun/Pistol_Sound_Cue.Pistol_Sound_Cue" _returnvalue_2 (struct) 1.0 1.0 0.0 null null null)
    (`GameplayStatics.SpawnEmitterAtLocation` "/Game/Materials/Weapon/Muzzle/P_muzzle.P_muzzle" _returnvalue_2 (`SceneComponent.K2_GetComponentRotation` (`self.Muzzle`)) (1.0 1.0 1.0) true "AutoRelease")
    (bind _outhit (`KismetSystemLibrary.LineTraceSingleForObjects` :`Start` _returnvalue_2 :`End` (+ (* (`SceneComponent.GetForwardVector` _muzzle_2) 5000) _returnvalue_2) :`ObjectTypes` (`|MakeArray` "ObjectTypeQuery9" :!type "EObjectTypeQuery Enum") :`DrawTime` 2.0))
    (bind (_bblockinghit _binitialoverlap _time _distance _location _impactpoint _normal _impactnormal _physmat _hitactor) (`GameplayStatics.BreakHitResult` _outhit))
    (`GameplayStatics.SpawnEmitterAtLocation` "/Game/Weapons/Particles/sparksParticle.sparksParticle" _impactpoint (struct) (1.0 1.0 1.0) true "AutoRelease")
    (`GameplayStatics.SpawnEmitterAtLocation` "/Game/Materials/Weapon/Materials_Particles/Bullet_01.Bullet_01" (`SceneComponent.K2_GetComponentLocation` _muzzle) (`SceneComponent.K2_GetComponentRotation` _muzzle))
    (bind _asaidrone (cast `AIDrone` _hitactor))
    (`I_Damageable.TakeDamage` _asaidrone 75.0)))

(fn `UserConstructionScript`)