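; Rocket projectile that explodes on its first hit and can home in on an AI drone.
; The hit fires a radial impulse, spawns explosion effect and sound, enables the AOE damage collision, then destroys the actor.
; HomingRocket targets the drone's mesh, or switches homing off when its health is zero.
; The AOE collision starts disabled, and the drone damage call is unwired, so this graph applies no damage.
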(event `self.ReceiveBeginPlay`
  (bind _aoedamage (`self.AOEDamage`))
  (`PrimitiveComponent.SetCollisionEnabled` _aoedamage "NoCollision")
  (`SceneComponent.SetVisibility` _aoedamage true false))

(event `self.CollisionComponent.OnComponentHit`
  (params (HitComponent :type "PrimitiveComponent Object Reference") (OtherActor :type "Actor Object Reference") (OtherComp :type "PrimitiveComponent Object Reference") (NormalImpulse :type "Vector Structure") (Hit :type "HitResult Structure (by ref)"))
  (bind _explosiveforce (`self.ExplosiveForce`))
  ;[1 1 1] Rocket Projectile functions
  (`/Engine/EditorBlueprintResources/StandardMacros.DoOnce` false
    (:`Completed`
      (`RadialForceComponent.FireImpulse` _explosiveforce)
      (`GameplayStatics.SpawnEmitterAtLocation` "/Game/Materials/Rocket_Projectile/P_Explosion.P_Explosion" (`SceneComponent.K2_GetComponentLocation` _explosiveforce) (struct) (1.0 1.0 1.0) true "AutoRelease")
      (`GameplayStatics.PlaySoundAtLocation` "/Game/Audio/SFX/Explosion02_Cue.Explosion02_Cue" (`SceneComponent.K2_GetComponentLocation` (`self.Sphere`)) (struct) 1.0 1.0 0.0 null null null) ; Play firing sound
      (`PrimitiveComponent.SetCollisionEnabled` (`self.AOEDamage`) "QueryAndPhysics")
      (`self.K2_DestroyActor`))))

(event `HomingRocket`
  (params (`Actor Target` :type "Actor Object Reference") (`Static Mesh Target` :type "StaticMeshActor Object Reference") (`Primitive Component Target` :type "PrimitiveComponent Object Reference") (AIDrone :type "AIDrone Object Reference"))
  (bind _projectile (`self.Projectile`))
  ;[1 1 1] Set Homing Missile
  (if (`KismetSystemLibrary.IsValid` AIDrone)
    (if (== (`AIDrone.health` AIDrone) 0.0)
      (set `ProjectileMovementComponent.bIsHomingProjectile` false _projectile)
      (else
        (set `ProjectileMovementComponent.HomingTargetComponent` (`Character.Mesh` AIDrone) _projectile)
        (set `ProjectileMovementComponent.bIsHomingProjectile` true _projectile)
        (set `ProjectileMovementComponent.HomingAccelerationMagnitude` 25000.0 _projectile)))))

(fn `UserConstructionScript`)