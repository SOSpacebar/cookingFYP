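; Shield weapon Blueprint that projects a collidable shield while the trigger is held, starting hidden with collision off.
; Pressing shows the projection, enables collision, plays a start sound and runs a timeline that drives its Z scale.
; Releasing plays an end sound and runs a second scale timeline, whose update hides the projection and disables collision after a short delay.
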(event `self.ReceiveBeginPlay`
  (bind _projection (`self.Projection`))
  ;[1 1 1] Hide Projection at the start
  (`self.SetSpawnMaterial`)
  (`SceneComponent.SetHiddenInGame` _projection true false)
  (`PrimitiveComponent.SetCollisionEnabled` _projection "NoCollision"))

(event `/Game/Weapons/Blueprints/GunInterface.IsTriggerPressed`
  (params (IsPressed :type Boolean))
  ;[1 1 1] Enable and disable shield functions
  (if IsPressed
    (set `self.IsShieldActive` true)
    (`self.SetActive` (`self.Projection`))
    (`GameplayStatics.PlaySoundAtLocation` "/Engine/EditorSounds/GamePreview/StartSimulate.StartSimulate" (`self.K2_GetActorLocation`) (struct) 1.0 1.0 0.0 null null null) ; Play firing sound
    (bind (_direction _scale_output) (`Timeline|Timeline_0_0` :!via `PlayFromStart`)
      (:`Update`
        (`SceneComponent.SetWorldScale3D` (`self.Projection`) (`KismetMathLibrary.MakeVector` 1.0 1.0 _scale_output))))
    (elif (`self.IsShieldActive`)
      (`GameplayStatics.PlaySoundAtLocation` "/Engine/EditorSounds/GamePreview/EndSimulate.EndSimulate" (`self.K2_GetActorLocation`) (struct) 1.0 1.0 0.0 null null null) ; Play firing sound
      (bind (_direction_2 _scale_output_2) (`Timeline|Timeline_1_0` :!via `PlayFromStart`)
        (:`Update`
          (`SceneComponent.SetWorldScale3D` (`self.Projection`) (`KismetMathLibrary.MakeVector` 1.0 1.0 _scale_output_2))
          (`KismetSystemLibrary.Delay` 0.2)
          (`self.SetInactive` (`self.Projection`))
          (set `self.IsShieldActive` false))))))

(fn `SetActive`
  (params (Projection :type "StaticMeshComponent Object Reference"))
  (`SceneComponent.SetHiddenInGame` Projection false false)
  (`PrimitiveComponent.SetCollisionEnabled` Projection "QueryAndPhysics"))

(fn `SetInactive`
  (params (Projection :type "StaticMeshComponent Object Reference"))
  (`SceneComponent.SetHiddenInGame` Projection true false)
  (`PrimitiveComponent.SetCollisionEnabled` Projection "NoCollision"))

(fn `UserConstructionScript`)