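; Rocket launcher interactable that marks a static mesh target and fires homing rockets at it.
; Pressing the trigger line-traces from the muzzle, stores the hit StaticMeshActor as the homing target and briefly highlights it through custom depth.
; Releasing the trigger spawns a rocket projectile at the muzzle, plays the firing sound and passes it the stored target, which persists when a later trace misses.
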(event `/Game/VirtualRealityBP/Blueprints/GunInterface.IsTriggerPressed`
  (params (IsPressed :type Boolean))
  (bind _muzzlelocation (`self.MuzzleLocation`))
  (bind _muzzlelocation_2 (`self.MuzzleLocation`))
  (bind _homingtarget (`self.HomingTarget`))
  (bind _returnvalue (`SceneComponent.K2_GetComponentLocation` _muzzlelocation_2))
  (bind _staticmeshcomponent (`StaticMeshActor.StaticMeshComponent` _homingtarget))
  ;[1 1 1] Rocket Functions
  (if IsPressed
    ;;[1 1 1] Targeting Laser
    (set `self.TriggeredForFire` true)
    (bind (_outhit _returnvalue_2) (`KismetSystemLibrary.LineTraceSingleForObjects` :`Start` _returnvalue :`End` (+ _returnvalue (* (`SceneComponent.GetForwardVector` _muzzlelocation_2) 5000.0)) :`ObjectTypes` (`self.ObjectsTarget`) :`DrawDebugType` "ForDuration"))
    (if _returnvalue_2
      (bind _asstatic_mesh_actor (cast `StaticMeshActor` (`.HitActor` (`GameplayStatics.BreakHitResult` _outhit))))
      (`/Engine/EditorBlueprintResources/StandardMacros.IsValid` _homingtarget
        (:`Is Valid`
          (`PrimitiveComponent.SetRenderCustomDepth` _staticmeshcomponent false))
        (:`Is Not Valid`
          _))
      (bind _output_get (set `self.HomingTarget` _asstatic_mesh_actor))
      (bind _staticmeshcomponent_2 (`StaticMeshActor.StaticMeshComponent` _output_get))
      (`PrimitiveComponent.SetRenderCustomDepth` _staticmeshcomponent_2 true)
      (`KismetSystemLibrary.Delay` 2.0)
      (`PrimitiveComponent.SetRenderCustomDepth` _staticmeshcomponent_2 false)
      (else
        (`/Engine/EditorBlueprintResources/StandardMacros.IsValid` _homingtarget
          (:`Is Valid`
            (`PrimitiveComponent.SetRenderCustomDepth` _staticmeshcomponent false)))))
    (else
      ;;[1 1 1] Fire Rocket
      (if (`self.TriggeredForFire`)
        (bind _returnvalue_3 (`|SpawnActorFromClass` "/Game/Interactables/RocketProjectile.RocketProjectile_C" (`KismetMathLibrary.MakeTransform` (`SceneComponent.K2_GetComponentLocation` _muzzlelocation) (`SceneComponent.K2_GetComponentRotation` _muzzlelocation)) "Undefined" "OverrideRootScale" null null))
        (`GameplayStatics.PlaySoundAtLocation` "/Game/Audio/GunFire_Cue.GunFire_Cue" (`self.K2_GetActorLocation`) (struct) 1.0 1.0 0.0 null null null) ; Play firing sound
        (set `self.TriggeredForFire` false)
        (`/Game/Interactables/RocketProjectile.HomingRocket` _returnvalue_3 null (`self.HomingTarget`) null)))))

(fn `UserConstructionScript`)