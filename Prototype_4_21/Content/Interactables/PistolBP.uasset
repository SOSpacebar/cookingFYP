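; Pistol Blueprint that fires a projectile when it receives a trigger press.
; IsTriggerPressed spawns a FirstPersonProjectile at the MuzzleLocation transform and plays a gunfire sound at the actor.
; A CanFire gate with two chained delays clears GunFiring and then re-enables firing, limiting the fire rate.
; Firing also prints a debug string and hides the Pistol component, which is not shown again here.
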(event `/Game/VirtualRealityBP/Blueprints/GunInterface.IsTriggerPressed`
  (params (IsPressed :type Boolean))
  (bind _muzzlelocation (`self.MuzzleLocation`))
  (if IsPressed
    (if (`self.canFire`)
      (set `self.GunFiring` true)
      (set `self.canFire` false)
      (`KismetSystemLibrary.PrintString` "fire")
      (`SceneComponent.SetHiddenInGame` (`self.Pistol`) true false)
      (`|SpawnActorFromClass` "/Game/Interactables/FirstPersonProjectile.FirstPersonProjectile_C" (`KismetMathLibrary.MakeTransform` (`SceneComponent.K2_GetComponentLocation` _muzzlelocation) (`SceneComponent.K2_GetComponentRotation` _muzzlelocation)) "Undefined" "OverrideRootScale" null null)
      (`GameplayStatics.PlaySoundAtLocation` "/Game/Audio/GunFire_Cue.GunFire_Cue" (`self.K2_GetActorLocation`) (struct) 1.0 1.0 0.0 null null null) ; Play firing sound
      (`KismetSystemLibrary.Delay` 0.2)
      (set `self.GunFiring` false)
      (`KismetSystemLibrary.Delay` 0.2)
      (set `self.canFire` true))))

(fn `UserConstructionScript`)