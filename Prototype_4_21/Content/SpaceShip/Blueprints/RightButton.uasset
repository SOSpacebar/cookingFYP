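; Right-hand push button on a spaceship control panel that sets the holder's chair location panel to 2 when fully pressed.
; An overlapping component drives the press: each tick its movement in the base's local Z, clamped to a maximum, offsets the button.
; Full depth fires once per press with a sound, and the button interpolates back when released.
; Its material shows active while the holder's panel value is 2.
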(event `self.Button.OnComponentBeginOverlap`
  (params (OverlappedComponent :type "PrimitiveComponent Object Reference") (OtherActor :type "Actor Object Reference") (OtherComp :type "PrimitiveComponent Object Reference") (OtherBodyIndex :type Integer) (bFromSweep :type Boolean) (SweepResult :type "HitResult Structure (by ref)"))
  ;[1 1 1] Pressing Button
  (`/Engine/EditorBlueprintResources/StandardMacros.IsValid` (`self.Overlapped Component`)
    (:`Is Not Valid`
      (bind _output_get (set `self.Overlapped Component` OtherComp))
      (set `self.Initial Location` (`SceneComponent.K2_GetComponentLocation` _output_get)))))

(event `self.Button.OnComponentEndOverlap`
  (params (OverlappedComponent :type "PrimitiveComponent Object Reference") (OtherActor :type "Actor Object Reference") (OtherComp :type "PrimitiveComponent Object Reference") (OtherBodyIndex :type Integer))
  ;[1 1 1] Pressing Button
  (if (== OtherComp (`self.Overlapped Component`))
    (set `self.Overlapped Component` null)))

(event `self.ReceiveTick`
  (params (DeltaSeconds :type "Float (single-precision)"))
  (bind _button (`self.Button`))
  (bind _buttonbase (`self.ButtonBase`))
  (bind (_returnvalue_x _returnvalue_y _returnvalue_z) (`KismetMathLibrary.BreakVector` (- (`KismetMathLibrary.InverseTransformLocation` (`SceneComponent.K2_GetComponentToWorld` _buttonbase) (`self.Initial Location`)) (`KismetMathLibrary.InverseTransformLocation` (`SceneComponent.K2_GetComponentToWorld` _buttonbase) (`SceneComponent.K2_GetComponentLocation` (`self.Overlapped Component`))))))
  ;[1 1 1] Button Update
  (`|ExecutionSequence`
    (:`then_0`
      (`/Engine/EditorBlueprintResources/StandardMacros.IsValid` (`self.Overlapped Component`)
        (:`Is Valid`
          (bind _output_get (set `self.BtnPressedAmt` (`KismetMathLibrary.FClamp` _returnvalue_z 0.0 (`self.MaxBtnPressedAmt`))))
          (bind _returnvalue (* _output_get -1.0))
          (`SceneComponent.K2_SetRelativeLocation` _button (`KismetMathLibrary.MakeVector` _returnvalue 0.0 _returnvalue) false false)
          ;[1 1 1] Action to do upon pressed
          ;;[1 1 1] Checks to run button once
          (if (== (`self.MaxBtnPressedAmt`) (`self.BtnPressedAmt`))
            (`/Engine/EditorBlueprintResources/StandardMacros.DoOnce` false :!label _label
              (:`Completed`
                (set `/Game/SpaceShip/Blueprints/ControlPanel_Chair.ChairLocation_Panel` 2 (`self.ButtonHolder`))
                (`GameplayStatics.PlaySoundAtLocation` "/Game/Audio/SpaceShip/Button_sound_cue.Button_sound_cue" (`SceneComponent.K2_GetComponentLocation` (`self.Button`)) (struct) 1.0 1.0 0.0 null null null)))
            (else
              (goto _label :!via `Reset`))))
        (:`Is Not Valid`
          (`SceneComponent.K2_SetRelativeLocation` _button (`KismetMathLibrary.VInterpTo` (`SceneComponent.RelativeLocation` (`self.Button`)) (0.0 0.0 0.0) DeltaSeconds) false false))))
    (:`then_1`
      (if (== (`/Game/SpaceShip/Blueprints/ControlPanel_Chair.ChairLocation_Panel` (`self.ButtonHolder`)) 2)
        (`PrimitiveComponent.SetMaterial` (`self.Button`) 0 "/Game/Materials/AirShip/Control_Panel_Materials/ControlPanel_Material_Active.ControlPanel_Material_Active")
        (else
          (`PrimitiveComponent.SetMaterial` (`self.Button`) 0 "/Game/Materials/AirShip/Control_Panel_Materials/ControlPanel_Material.ControlPanel_Material"))))))

(fn `UserConstructionScript`)