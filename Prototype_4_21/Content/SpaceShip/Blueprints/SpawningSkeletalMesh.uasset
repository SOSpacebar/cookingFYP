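; Skeletal mesh actor in the SpaceShip content that animates its materials' "fadeout" parameter when spawning and despawning.
; SetSpawnMaterial builds the dynamic material instances that both timelines drive.
; Spawn holds the mesh as WorldStatic during its fade, then switches it to a custom collision channel.
; TriggerSpawn disables overlaps and flip-flops between playing a fade that destroys the actor on finish and reversing it.
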(event `self.ReceiveBeginPlay`)

(event `TriggerSpawn`
  (set `PrimitiveComponent.bGenerateOverlapEvents` false (`self.TheSkeletalMesh`))
  (`/Engine/EditorBlueprintResources/StandardMacros.FlipFlop`
    (:`A`
      (bind (_direction _newtrack_0) (`Timeline|Timeline_0` :!via `PlayFromStart` :!label _label)
        (:`Update`
          (for _array_element (`self.DynamicMaterial`)
            (`MaterialInstanceDynamic.SetScalarParameterValue` _array_element "fadeout" (`KismetMathLibrary.Lerp` 1.0 0.0 _newtrack_0))))
        (:`Finished`
          (`self.K2_DestroyActor`))))
    (:`B`
      (goto _label :!via `ReverseFromEnd`))))

(event `Spawn`
  (bind _theskeletalmesh (`self.TheSkeletalMesh`))
  (`PrimitiveComponent.SetCollisionObjectType` _theskeletalmesh "ECC_WorldStatic")
  (for _array_element (`self.DynamicMaterial`)
    (`MaterialInstanceDynamic.SetScalarParameterValue` _array_element "fadeout" 0.0)
    (bind (_direction _newtrack_0) (`Timeline|Timeline_1` :!via `PlayFromStart`)
      (:`Update`
        (for _array_element_2 (`self.DynamicMaterial`)
          (`MaterialInstanceDynamic.SetScalarParameterValue` _array_element_2 "fadeout" (`KismetMathLibrary.Lerp` 1.0 0.0 _newtrack_0))))
      (:`Finished`
        (`PrimitiveComponent.SetCollisionObjectType` _theskeletalmesh "ECC_GameTraceChannel1")))))

(fn `SetSpawnMaterial`
  (bind _theskeletalmesh (`self.TheSkeletalMesh`))
  (for (_array_element _array_index) (`MeshComponent.GetMaterials` _theskeletalmesh)
    (bind _returnvalue (`PrimitiveComponent.CreateDynamicMaterialInstance` _theskeletalmesh _array_index _array_element "None"))
    (`KismetArrayLibrary.Array_Add` (`self.DynamicMaterial`) _returnvalue)))

(fn `UserConstructionScript`)