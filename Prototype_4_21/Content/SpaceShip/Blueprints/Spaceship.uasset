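; Player spaceship actor that carries the scripted mission from world reveal through boss approach to the restartable ending.
; GameManager scenario events trigger timelines that move Airship along successive splines, scale the world, toggle warp, play audio and launch the next event.
; Tick slides and rotates the chair between cockpit, left and right stations via a back point, following the control panel's selection.
; Overlaps handle emergency box release, projectile hurt UI and logo/credits cycling.
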(event `self.ReceiveTick`
  (params (DeltaSeconds :type "Float (single-precision)"))
  (`self.MoveToPosition` DeltaSeconds)
  (`SceneComponent.K2_AddLocalRotation` (`self.WireframeShip`) (struct :`Yaw` 1.0) false false)
  (`SceneComponent.K2_AddLocalRotation` (`self.WireframeBuilding`) (struct :`Yaw` 1.0) false false))

(event `self.ReceiveBeginPlay`
  (bind _warp (`self.Warp`))
  (bind _controlpanel_chair (`self.ControlPanel_Chair`))
  (bind _warp_2 (`self.Warp`))
  (bind _logo (`self.Logo`))
  ;[1 1 1] Event Listener
  (set `self.ChairButton_Cockpit_Child` _controlpanel_chair)
  (set `self.ChairButton_Right_Child` _controlpanel_chair)
  (set `self.ChairButton_Left_Child` _controlpanel_chair)
  (bind _asgame_manager (cast `GameManager` (`GameplayStatics.GetGameMode`)))
  (add `GameManager.onScenarioComplete` _asgame_manager (delegate `StartShip`))
  (bind _returnvalue (`GameplayStatics.SpawnSound2D` "/Game/Audio/BGM/FYP_Start_Bgm2_Cue.FYP_Start_Bgm2_Cue" 1.0 1.0 0.0 null))
  (`SceneComponent.SetWorldScale3D` (`/Game/SpaceShip/Blueprints/WorldScaler.DefaultSceneRoot` (`self.TheWorldScalar`)) (0.0 0.0 0.0))
  (bind _asemergency_box (cast `/Game/SpaceShip/Blueprints/EmergencyBox` (`ChildActorComponent.ChildActor` (`self.EmergencyBox`))))
  (set `/Game/SpaceShip/Blueprints/EmergencyBox.TheSpaceship` self _asemergency_box)
  (`self.runNextScriptedMovement` :!label _label)
  (switch `int` (`KismetMathLibrary.Conv_ByteToInt` (stale `StartShip` _scenario))
    (:`1`
      (bind (_direction _newtrack_0) (`Timeline|worldscaling`)
        (:`Update`
          (`SceneComponent.SetWorldScale3D` (`/Game/SpaceShip/Blueprints/WorldScaler.DefaultSceneRoot` (`self.TheWorldScalar`)) (`KismetMathLibrary.MakeVector` _newtrack_0 _newtrack_0 _newtrack_0))
          (`self.animationAlphaToWorldTransform` _newtrack_0))
        (:`Finished`
          (`/Engine/EditorBlueprintResources/StandardMacros.IncrementInt` (`self.currentSequence`)
            (:`  `
              (`self.runNextScriptedMovement`)
              (`ActorComponent.SetComponentTickEnabled` _warp_2 false)
              (`SceneComponent.SetHiddenInGame` _warp_2 true false)
              (bind (_direction_2 _animationalpha) (`Timeline|Timeline_0`)
                (:`Update`
                  (`self.animationAlphaToWorldTransform` _animationalpha))
                (:`Finished`
                  (`/Engine/EditorBlueprintResources/StandardMacros.IncrementInt` (`self.currentSequence`)
                    (:`  `
                      (bind _asgame_manager_2 (cast `GameManager` (`GameplayStatics.GetGameMode`)))
                      (`GameManager.RunEvent` _asgame_manager_2 2)
                      (`GameplayStatics.PlaySound2D` "/Game/Audio/Dialogue/Enemies_Approaching_Cue.Enemies_Approaching_Cue" 1.0 1.0 0.0 null null))))))))))
    (:`4`
      (bind (_direction_3 _newtrack_0_2) (`Timeline|Timeline_1`)
        (:`Update`
          (`self.animationAlphaToWorldTransform` _newtrack_0_2))
        (:`Finished`
          (`/Engine/EditorBlueprintResources/StandardMacros.IncrementInt` (`self.currentSequence`)
            (:`  `
              (bind _asgame_manager_3 (cast `GameManager` (`GameplayStatics.GetGameMode`)))
              (`GameManager.RunEvent` _asgame_manager_3 5))))))
    (:`6`
      (`GameplayStatics.PlaySound2D` "/Game/Audio/Dialogue/Boss_approaching_Cue.Boss_approaching_Cue" 1.0 1.0 0.0 null null)
      (bind (_direction_4 _newtrack_0_3) (`Timeline|Timeline_2`)
        (:`Update`
          (`self.animationAlphaToWorldTransform` _newtrack_0_3))
        (:`Finished`
          (`/Engine/EditorBlueprintResources/StandardMacros.IncrementInt` (`self.currentSequence`)
            (:`  `
              (bind _asgame_manager_4 (cast `GameManager` (`GameplayStatics.GetGameMode`)))
              (`GameManager.RunEvent` _asgame_manager_4 7)
              (`GameplayStatics.PlaySound2D` "/Game/Audio/Dialogue/Boss_appear_Cue.Boss_appear_Cue" 1.0 1.0 0.0 null null)
              (`AudioComponent.AdjustVolume` _returnvalue 10.0 0.0)
              (`GameplayStatics.PlaySound2D` "/Game/Audio/BGM/boss_techno_Cue.boss_techno_Cue" 1.0 1.0 0.0 null null))))))
    (:`8`
      (`GameplayStatics.PlaySound2D` "/Game/Audio/Dialogue/Mission_accomplish_Cue.Mission_accomplish_Cue" 1.0 1.0 0.0 null null)
      (`ActorComponent.SetComponentTickEnabled` _warp true)
      (`SceneComponent.SetHiddenInGame` _warp false false)
      (bind (_direction_5 _newtrack_0_4) (`Timeline|Timeline_3`)
        (:`Update`
          (`self.animationAlphaToWorldTransform` _newtrack_0_4)
          (bind _returnvalue_2 (- 1.0 _newtrack_0_4))
          (`SceneComponent.SetWorldScale3D` (`/Game/SpaceShip/Blueprints/WorldScaler.DefaultSceneRoot` (`self.TheWorldScalar`)) (`KismetMathLibrary.MakeVector` _returnvalue_2 _returnvalue_2 _returnvalue_2)))
        (:`Finished`
          (set `self.IsGameOver` true)
          (`TextRenderComponent.K2_SetText` (`self.Credits`) (`KismetTextLibrary.Conv_StringToText` "Press here to<br>restart game"))
          (if (`SceneComponent.IsVisible` _logo)
            (`SceneComponent.SetVisibility` _logo false false)))))))

(event `StartShip`
  (params (_scenario :type Byte))
  ;[1 1 1] Event Listener
  (if (or (== _scenario 1) (== _scenario 4) (== _scenario 6) (== _scenario 8))
    (goto _label)))

(event `self.Sphere.OnComponentBeginOverlap`
  (params (OverlappedComponent :type "PrimitiveComponent Object Reference") (OtherActor :type "Actor Object Reference") (OtherComp :type "PrimitiveComponent Object Reference") (OtherBodyIndex :type Integer) (bFromSweep :type Boolean) (SweepResult :type "HitResult Structure (by ref)"))
  (bind _asemergency_box (cast `/Game/SpaceShip/Blueprints/EmergencyBox` (`ChildActorComponent.ChildActor` (`self.EmergencyBox`))))
  (`/Game/SpaceShip/Blueprints/EmergencyBox.ReleaseLock` _asemergency_box)
  (`GameplayStatics.PlaySoundAtLocation` "/Game/Audio/SpaceShip/Button_sound_cue.Button_sound_cue" (`SceneComponent.K2_GetComponentLocation` OverlappedComponent) (struct) 1.0 1.0 0.0 null null null))

(event `self.HitBox.OnComponentBeginOverlap`
  (params (OverlappedComponent :type "PrimitiveComponent Object Reference") (OtherActor :type "Actor Object Reference") (OtherComp :type "PrimitiveComponent Object Reference") (OtherBodyIndex :type Integer) (bFromSweep :type Boolean) (SweepResult :type "HitResult Structure (by ref)"))
  (cast `/Game/AI/BluePrint/BP_Projectile` OtherActor)
  (bind _returnvalue (`|CreateWidget` "/Game/UI/BluePrint/HurtUI.HurtUI_C"))
  (`UserWidget.AddToViewport` _returnvalue 0))

(event `self.NetsCollider.OnComponentBeginOverlap`
  (params (OverlappedComponent :type "PrimitiveComponent Object Reference") (OtherActor :type "Actor Object Reference") (OtherComp :type "PrimitiveComponent Object Reference") (OtherBodyIndex :type Integer) (bFromSweep :type Boolean) (SweepResult :type "HitResult Structure (by ref)"))
  (bind _logo (`self.Logo`))
  (bind _netscollider (`self.NetsCollider`))
  (if (`self.IsGameOver`)
    (bind _returnvalue (`GameplayStatics.GetCurrentLevelName` true))
    (`GameplayStatics.OpenLevel` (`KismetStringLibrary.Conv_StringToName` _returnvalue))
    (else
      (`GameplayStatics.PlaySoundAtLocation` "/Game/Audio/SpaceShip/Button_sound_cue.Button_sound_cue" (`SceneComponent.K2_GetComponentLocation` OverlappedComponent) (struct) 1.0 1.0 0.0 null null null)
      (if (`SceneComponent.IsVisible` _logo)
        (`SceneComponent.SetVisibility` _logo false false)
        (`TextRenderComponent.K2_SetText` (`self.Credits`) (`self.ArtistCredits`))
        (set `PrimitiveComponent.bGenerateOverlapEvents` false _netscollider :!label _label_2)
        (`KismetSystemLibrary.Delay` 1.0)
        (set `PrimitiveComponent.bGenerateOverlapEvents` true _netscollider)
        (elif (== (`TextRenderComponent.Text` (`self.Credits`)) (`self.ArtistCredits`))
          (`TextRenderComponent.K2_SetText` (`self.Credits`) (`self.ProgrammerCredits`))
          (goto _label_2)
          (else
            (`TextRenderComponent.K2_SetText` (`self.Credits`) (`KismetTextLibrary.Conv_StringToText` ""))
            (`SceneComponent.SetVisibility` (`self.Logo`) true false)))))))

(fn `AdjustLights`
  (params (LightIntensity :type "Float (double-precision)"))
  (bind _lightintensityvalues (`self.LightIntensityValues`))
  (`LightComponent.SetIntensity` (`self.PointLight`) (* LightIntensity (`|GetArrayItem` _lightintensityvalues)))
  (`LightComponent.SetIntensity` (`self.PointLight1`) (* LightIntensity (`|GetArrayItem` _lightintensityvalues 1)))
  (`LightComponent.SetIntensity` (`self.PointLight2`) (* LightIntensity (`|GetArrayItem` _lightintensityvalues 2)))
  (`LightComponent.SetIntensity` (`self.PointLight3`) (* LightIntensity (`|GetArrayItem` _lightintensityvalues 3))))

(fn `animationAlphaToWorldTransform`
  (params (animationAlpha :type "Float (double-precision)"))
  (bind _currentspline (`self.currentSpline`))
  (bind _returnvalue (* animationAlpha (`SplineComponent.GetSplineLength` _currentspline)))
  (`SceneComponent.K2_SetWorldTransform` (`self.airship`) (`KismetMathLibrary.MakeTransform` (`SplineComponent.GetLocationAtDistanceAlongSpline` _currentspline _returnvalue "World") (`SplineComponent.GetRotationAtDistanceAlongSpline` _currentspline _returnvalue "World")) false false))

(fn `MoveToBack`
  (bind _errortolerance (`self.ErrorTolerance`))
  (bind _chair (`self.Chair`))
  (bind (_relativelocation_x _relativelocation_y) (`KismetMathLibrary.BreakVector` (`SceneComponent.RelativeLocation` (`self.Chair`))))
  (bind (_relativelocation_x_2 _relativelocation_y_2) (`KismetMathLibrary.BreakVector` (`SceneComponent.RelativeLocation` (`self.Chair`))))
  (bind (_relativelocation_x_3 _relativelocation_y_3) (`KismetMathLibrary.BreakVector` (`SceneComponent.RelativeLocation` (`self.Back`))))
  (bind _relativelocation (`SceneComponent.RelativeLocation` (`self.Back`)))
  (bind (_relativelocation_x_4 _relativelocation_y_4) (`KismetMathLibrary.BreakVector` (`SceneComponent.RelativeLocation` (`self.Chair`))))
  (bind (_relativelocation_x_5 _relativelocation_y_5) (`KismetMathLibrary.BreakVector` (`SceneComponent.RelativeLocation` (`self.Chair`))))
  (if (`KismetMathLibrary.NearlyEqual_FloatFloat` _relativelocation_y_4 0.0 _errortolerance)
    (set `self.OriginLocation` 0)
    (`SceneComponent.K2_AddRelativeLocation` (`self.Chair`) (* (* (`KismetMathLibrary.Normal` (- (`SceneComponent.RelativeLocation` (`self.Back`)) (`SceneComponent.RelativeLocation` (`self.Chair`)))) 100.0) (`GameplayStatics.GetWorldDeltaSeconds`)) false false :!label _label)
    (switch `int` (`self.OriginLocation`)
      (:`0`
        (if (< _relativelocation_x_2 _relativelocation_x_3)
          (`SceneComponent.K2_SetRelativeLocation` _chair _relativelocation false false)))
      (:`1`
        (if (> _relativelocation_y_2 _relativelocation_y_3)
          (`SceneComponent.K2_SetRelativeLocation` _chair _relativelocation false false)))
      (:`2`
        (if (< _relativelocation_y_2 _relativelocation_y_3)
          (`SceneComponent.K2_SetRelativeLocation` _chair _relativelocation false true))))
    (elif (< _relativelocation_y (* -1 _errortolerance))
      (set `self.OriginLocation` 1)
      (goto _label)
      (elif (> _relativelocation_y_5 _errortolerance)
        (set `self.OriginLocation` 2)
        (goto _label)
        (else
          (`KismetSystemLibrary.DrawDebugString` (0.0 0.0 0.0) "cannot find origin location" null))))))

(fn `MoveToPosition`
  (params (delta :type "Float (double-precision)"))
  (locals (NewLocalVar_0 :type "Float (double-precision)"))
  (bind _cockpit (`self.Cockpit`))
  (bind _cockpit_2 (`self.Cockpit`))
  (bind _left (`self.Left`))
  (bind _right (`self.Right`))
  (bind _errortolerance (`self.ErrorTolerance`))
  (bind _chair (`self.Chair`))
  (bind _errortolerance_2 (`self.ErrorTolerance`))
  (bind _chair_2 (`self.Chair`))
  (bind _chair_3 (`self.Chair`))
  (bind _chair_4 (`self.Chair`))
  (bind _chair_5 (`self.Chair`))
  (bind _chair_6 (`self.Chair`))
  (bind _chair_7 (`self.Chair`))
  (bind (_relativelocation_x _relativelocation_y) (`KismetMathLibrary.BreakVector` (`SceneComponent.RelativeLocation` _right)))
  (bind (_relativerotation_roll _relativerotation_pitch _relativerotation_yaw) (`KismetMathLibrary.BreakRotator` (`SceneComponent.RelativeRotation` _chair_7)))
  (bind _relativelocation_x_2 (`KismetMathLibrary.BreakVector` (`SceneComponent.RelativeLocation` (`self.Back`))))
  (bind _relativelocation (`SceneComponent.RelativeLocation` (`self.Right`)))
  (bind _relativelocation_2 (`SceneComponent.RelativeLocation` _chair_7))
  (bind (_relativelocation_x_3 _relativelocation_y_2) (`KismetMathLibrary.BreakVector` (`SceneComponent.RelativeLocation` (`self.Chair`))))
  (bind _relativelocation_x_4 (`KismetMathLibrary.BreakVector` (`SceneComponent.RelativeLocation` _chair_4)))
  (bind _relativelocation_x_5 (`KismetMathLibrary.BreakVector` (`SceneComponent.RelativeLocation` _cockpit_2)))
  (bind _relativelocation_x_6 (`KismetMathLibrary.BreakVector` (`SceneComponent.RelativeLocation` _chair_2)))
  (bind (_relativerotation_roll_2 _relativerotation_pitch_2 _relativerotation_yaw_2) (`KismetMathLibrary.BreakRotator` (`SceneComponent.RelativeRotation` _chair_3)))
  (bind _relativelocation_x_7 (`KismetMathLibrary.BreakVector` (`SceneComponent.RelativeLocation` _cockpit)))
  (bind (_relativelocation_x_8 _relativelocation_y_3) (`KismetMathLibrary.BreakVector` (`SceneComponent.RelativeLocation` (`self.Chair`))))
  (bind (_relativerotation_roll_3 _relativerotation_pitch_3 _relativerotation_yaw_3) (`KismetMathLibrary.BreakRotator` (`SceneComponent.RelativeRotation` _chair)))
  (bind _relativelocation_3 (`SceneComponent.RelativeLocation` (`self.Left`)))
  (bind _relativelocation_4 (`SceneComponent.RelativeLocation` _chair))
  (bind (_relativelocation_x_9 _relativelocation_y_4) (`KismetMathLibrary.BreakVector` (`SceneComponent.RelativeLocation` _chair_5)))
  (bind (_relativelocation_x_10 _relativelocation_y_5) (`KismetMathLibrary.BreakVector` (`SceneComponent.RelativeLocation` _left)))
  (bind (_relativelocation_x_11 _relativelocation_y_6) (`KismetMathLibrary.BreakVector` (`SceneComponent.RelativeLocation` (`self.Chair`))))
  (bind _relativelocation_x_12 (`KismetMathLibrary.BreakVector` (`SceneComponent.RelativeLocation` (`self.Back`))))
  (bind (_relativerotation_roll_4 _relativerotation_pitch_4 _relativerotation_yaw_4) (`KismetMathLibrary.BreakRotator` (`SceneComponent.RelativeRotation` _chair_3)))
  (bind (_relativerotation_roll_5 _relativerotation_pitch_5 _relativerotation_yaw_5) (`KismetMathLibrary.BreakRotator` (`SceneComponent.RelativeRotation` _chair_2)))
  (bind (_relativelocation_x_13 _relativelocation_y_7) (`KismetMathLibrary.BreakVector` (`SceneComponent.RelativeLocation` _chair_6)))
  (bind _ascontrol_panel_chair (cast `/Game/SpaceShip/Blueprints/ControlPanel_Chair` (`ChildActorComponent.ChildActor` (`self.ControlPanel_Chair`))))
  (switch `int` (`/Game/SpaceShip/Blueprints/ControlPanel_Chair.ChairLocation_Panel` _ascontrol_panel_chair)
    (:`0`
      (if (`KismetMathLibrary.NearlyEqual_FloatFloat` _relativelocation_y_6 0.0 (`self.ErrorTolerance`))
        (if (`KismetMathLibrary.NearlyEqual_FloatFloat` _relativerotation_yaw_5 0.0 (`self.ErrorTolerance`))
          (if (< _relativelocation_x_6 _relativelocation_x_7)
            (`SceneComponent.K2_AddRelativeLocation` _chair_2 (* (* (`KismetMathLibrary.Normal` (- (`SceneComponent.RelativeLocation` _cockpit) (`SceneComponent.RelativeLocation` _chair_2))) 100.0) (`GameplayStatics.GetWorldDeltaSeconds`)) false false)
            (if (> _relativelocation_x_4 _relativelocation_x_5)
              (`SceneComponent.K2_SetRelativeLocation` _chair_4 (`SceneComponent.RelativeLocation` _cockpit_2) false false)))
          (else
            ;[1 1 1] Which direction to rotate
            (if (< _relativerotation_yaw_5 0.0)
              (`SceneComponent.K2_AddLocalRotation` _chair_2 (`KismetMathLibrary.MakeRotator` 0.0 0.0 1.0) false false)
              (if (> _relativerotation_yaw_4 0.0)
                (`SceneComponent.K2_SetRelativeRotation` :`self` _chair_3))
              (else
                (`SceneComponent.K2_AddLocalRotation` _chair_3 (`KismetMathLibrary.MakeRotator` 0.0 0.0 (* (`GameplayStatics.GetWorldDeltaSeconds`) -100.0)) false false)
                (if (< _relativerotation_yaw_2 0.0)
                  (`SceneComponent.K2_SetRelativeRotation` :`self` _chair_3))))))
        (else
          (`self.MoveToBack`))))
    (:`1`
      (if (or (> _relativelocation_x_8 (+ _relativelocation_x_12 _errortolerance_2)) (> _relativelocation_y_3 _errortolerance_2))
        (`self.MoveToBack`)
        (elif (> _relativerotation_yaw_3 -90.0)
          (`SceneComponent.K2_AddLocalRotation` _chair (`KismetMathLibrary.MakeRotator` 0.0 0.0 (* (`GameplayStatics.GetWorldDeltaSeconds`) -100.0)) false false)
          (elif (not (== _relativelocation_4 _relativelocation_3 :`ErrorTolerance` 0.1))
            (`SceneComponent.K2_AddRelativeLocation` _chair (* (* (`KismetMathLibrary.Normal` (- _relativelocation_3 _relativelocation_4)) 100.0) (`GameplayStatics.GetWorldDeltaSeconds`)) false false)
            (if (< _relativelocation_y_4 _relativelocation_y_5)
              (`SceneComponent.K2_SetRelativeLocation` _chair_5 (`SceneComponent.RelativeLocation` _left) false false))))))
    (:`2`
      (if (or (> _relativelocation_x_3 (+ _relativelocation_x_2 _errortolerance)) (< _relativelocation_y_2 (* -1 _errortolerance)))
        (`self.MoveToBack`)
        (elif (< _relativerotation_yaw 90.0)
          (`SceneComponent.K2_AddLocalRotation` _chair_7 (`KismetMathLibrary.MakeRotator` 0.0 0.0 (* (`GameplayStatics.GetWorldDeltaSeconds`) 100.0)) false false)
          (elif (not (== _relativelocation_2 _relativelocation :`ErrorTolerance` 0.1))
            (`SceneComponent.K2_AddRelativeLocation` _chair_7 (* (* (`KismetMathLibrary.Normal` (- _relativelocation _relativelocation_2)) 100.0) (`GameplayStatics.GetWorldDeltaSeconds`)) false false)
            (if (> _relativelocation_y_7 _relativelocation_y)
              (`SceneComponent.K2_SetRelativeLocation` _chair_6 (`SceneComponent.RelativeLocation` _right) false false))))))))

(fn `runNextScriptedMovement`
  (locals (currentTimeline :type "TimelineComponent Object Reference"))
  (switch `int` (`self.currentSequence`)
    (:`0`
      (set `self.currentSpline` (`self.Spline`)))
    (:`1`
      (set `self.currentSpline` (`self.Spline0`)))
    (:`2`
      (set `self.currentSpline` (`self.Spline1`)))
    (:`3`
      (set `self.currentSpline` (`self.Spline3`)))
    (:`4`
      (set `self.currentSpline` (`self.Spline4`)))))

(fn `UserConstructionScript`)