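; ControlPanel_Chair is a spaceship chair control panel Blueprint that hosts three buttons: right, left and cockpit.
; On BeginPlay it casts each button's child actor to its button class and sets itself as that button's ButtonHolder.
; The casts run in sequence, so a failed cast leaves the remaining buttons unlinked.
; The panel contains no press handling or other active logic, only this back-reference wiring.
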(event `self.ReceiveBeginPlay`
  (bind _asright_button (cast `/Game/SpaceShip/Blueprints/RightButton` (`ChildActorComponent.ChildActor` (`self.RightButton`))))
  (set `/Game/SpaceShip/Blueprints/RightButton.ButtonHolder` self _asright_button)
  (bind _asleft_button (cast `/Game/SpaceShip/Blueprints/LeftButton` (`ChildActorComponent.ChildActor` (`self.LeftButton`))))
  (set `/Game/SpaceShip/Blueprints/LeftButton.Button holder ` self _asleft_button)
  (bind _ascockpit_button (cast `/Game/SpaceShip/Blueprints/CockpitButton` (`ChildActorComponent.ChildActor` (`self.CockpitButton`))))
  (set `/Game/SpaceShip/Blueprints/CockpitButton.Button holder` self _ascockpit_button))

(fn `UserConstructionScript`)